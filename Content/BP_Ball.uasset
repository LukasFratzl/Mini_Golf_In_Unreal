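; BP_Ball is a ball actor that handles mouse drag feedback on screen.
; Left click shows and hides the drag circle on the BP_MGHud found at BeginPlay, keeping the cursor visible.
; Tick traces from the camera through the cursor, lerps between the sphere and hit location, then projects that point into viewport space for MgWidget's LerpPosition.
; No ball movement is implemented, and UpdateBallUI is empty.
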(event EventBeginPlay
  (bind _outactors (Actor|GetAllActorsOfClass "/Game/BP_MGHud.BP_MGHud_C"))
  (Variables|Default|SetMGHud (Utilities|Array|Get(acopy) _outactors)))

(event Collision|EventActorBeginOverlap
  (params (OtherActor :type Actor%20Object%20Reference)))

(event EventTick
  (params (DeltaSeconds :type Float%20%28single-precision%29))
  (bind _returnvalue (Game|GetPlayerCameraManager 0))
  (bind _returnvalue_2 (Class|GameplayStatics|GetPlayerControllerfromID))
  (bind _mgwidget (Variables|Default|GetmgWidget))
  (bind _returnvalue_3 (Transformation|GetActorLocation _returnvalue))
  (bind (_locationx _locationy) (Game|Player|GetMousePosition _returnvalue_2))
  (bind _outhit (Collision|LineTraceByChannel _returnvalue_3 (* (- (.WorldPosition (Class|GameplayStatics|DeprojectScreentoWorld _returnvalue_2 (Math|Vector2D|MakeVector2D _locationx _locationy))) _returnvalue_3) 1e+05) "TraceTypeQuery1" false 0 "None"))
  (if (!= _mgwidget 0)
    (Variables|/Game/W_MiniGolfHud.W_MiniGolfHud_C|SetlerpPosition _mgwidget (Class|SlateBlueprintLibrary|ScreentoViewport (.ScreenPosition (Class|GameplayStatics|ProjectWorldtoScreen _returnvalue_2 (Math|Vector|Lerp(Vector) (Transformation|GetWorldLocation (Variables|Default|GetSphere)) (.location _outhit) (Variables|Default|GetAlpha)) false))))))

(event Input|ActionEvents|InputActionLeftClick
  (params (Key :type Key%20Structure :default "None"))
  (bind _returnvalue (Class|GameplayStatics|GetPlayerControllerfromID))
  (:Pressed
    (Development|PrintString "Clicked")
    (Class|Image|SetOpacity (Variables|/Game/BP_MGHud.BP_MGHud_C|GetDrag%20Circle (Variables|Default|GetMGHud)) 1e+02)
    (Variables|/Script/Engine.PlayerController|SetbShowMouseCursor _returnvalue true))
  (:Released
    (Development|PrintString "Released")
    (Class|Image|SetOpacity (Variables|/Game/BP_MGHud.BP_MGHud_C|GetDrag%20Circle (Variables|Default|GetMGHud)) 0.0)
    (Variables|/Script/Engine.PlayerController|SetbShowMouseCursor _returnvalue true)))

(fn ConstructionScript)

(fn UpdateBallUI)